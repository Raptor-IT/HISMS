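; Constituency manager that spawns the game's constituency markers as instances on a single instanced static mesh component at BeginPlay.
; It reads Lies of Polls data table rows by index, placing each instance at the row's local X/Y/Z with a shared rotation offset and unit scale.
; The loop runs to MaxConstituencies, but indices from 650 upward only print a completion message.
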(event EventBeginPlay
  (for _index (range 0 (- (Variables|Default|GetMax%20Constituencies) 1))
    (if (>= _index 650)
      (Development|PrintString "All consticuencies Created")
      (else
        (bind _returnvalue (Utilities|GetDataTableRow "/Game/Core/Data/LiesOfPolls_-_Data_Table_-_Sheet1__2_.LiesOfPolls_-_Data_Table_-_Sheet1__2_" (Utilities|String|StringToName (Utilities|String|ToString(Integer) _index)))
          (:then
            (Variables|Default|SetName (.Name (Utilities|Struct|BreakF_Constituencies _returnvalue)))
            (bind _output_get (Variables|Default|SetLocation (Math|Vector|MakeVector (.X (Utilities|Struct|BreakF_Constituencies _returnvalue)) (.Y (Utilities|Struct|BreakF_Constituencies _returnvalue)) (.Z (Utilities|Struct|BreakF_Constituencies _returnvalue)))))
            (bind _output_get_2 (Variables|Default|SetTransform (Math|Transform|MakeTransform _output_get (Variables|Default|GetRotaion%20Offset) "1.000000,1.000000,1.000000")))
            (Components|InstancedStaticMesh|AddInstance (Variables|Default|GetConstituencieISM) _output_get_2 false)))))))

(fn ConstructionScript)