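; BP_TileManager builds a square grid of randomized grass, sand and mountain tiles on BeginPlay.
; The construction script derives the row length from the square root of the tile count and sets each terrain's material color.
; BiuldTiles steps through grid positions, maps a seeded stream roll to a terrain type, then adds the tile to that type's instanced static mesh component and appends a terrain tag.
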(event EventBeginPlay
  (CallFunction|BiuldTiles))

(event Collision|EventActorBeginOverlap
  (params (OtherActor :type Actor%20Object%20Reference)))

(event EventTick
  (params (DeltaSeconds :type Float%20%28single-precision%29)))

(fn ConstructionScript
  ;[1 1 1] Set Tile Length
  (Variables|Default|SetTileLineLength (Math|Float|Truncate (Math|Float|Sqrt (Math|Conversions|ToFloat(Integer) (Variables|Default|GetTileMaxLength)))))
  ;[1 1 1] Sete meterial instance colour
  (Rendering|Material|SetVectorParameterValueonMaterials (Variables|Default|GetGrassISM) "TileType" "0.000000,1.000000,0.000000")
  (Rendering|Material|SetVectorParameterValueonMaterials (Variables|Default|GetSandISM) "TileType" "1.000000,1.000000,0.000000")
  (Rendering|Material|SetVectorParameterValueonMaterials (Variables|Default|GetMountainISM) "TileType" "0.338500,0.100000,0.000000"))

(fn BiuldTiles
  (for _index (range 0 (- (Variables|Default|GetTileMaxLength) 1))
    (Variables|Default|SetStreamSeed (Math|Random|RandomIntegerinRangefromStream (Variables|Default|GetSeed) 0 10))
    (if (== (Math|Integer|%(Integer) _index (Variables|Default|GetTileLineLength)) 0)
      (bind _output_get (Variables|Default|SetTileLocation (Math|Vector|MakeVector (+ (.x (.Location (Math|Transform|BreakTransform (Math|Transform|MakeTransform (Variables|Default|GetTileLocation))))) 1e+02) (- (Variables|Default|GetTileLineLength) (Variables|Default|GetIncreaseY)) 0.0)))
      (CallFunction|GenerateTileTerrain)
      (CallFunction|AddISM (Math|Conversions|ToTransform(Vector) _output_get))
      (else
        (bind _output_get_2 (Variables|Default|SetTileLocation (- (Variables|Default|GetTileLocation) (Math|Vector|MakeVector (Variables|Default|GetIncreaseX) (+ (Variables|Default|GetIncreaseY) 1e+02) 0.0))))
        (CallFunction|GenerateTileTerrain)
        (CallFunction|AddISM (Math|Conversions|ToTransform(Vector) _output_get_2))))))

(fn GenerateTileTerrain
  (bind _streamseed (Variables|Default|GetStreamSeed))
  (if (<= _streamseed 3)
    (Variables|Default|SetTerrainType "NewEnumerator0")
    (elif (>= _streamseed 7)
      (Variables|Default|SetTerrainType "NewEnumerator2")
      (else
        (Variables|Default|SetTerrainType "NewEnumerator1")))))

(fn AddISM
  (params (InstanceTransform :type Transform%20%28by%20ref%29))
  (bind _grassism (Variables|Default|GetGrassISM))
  (bind _sandism (Variables|Default|GetSandISM))
  (bind _mountainism (Variables|Default|GetMountainISM))
  (switch Utilities|FlowControl|Switch|SwitchonE_TerrainTileType (Variables|Default|GetTerrainType)
    (:NewEnumerator0
      (Components|InstancedStaticMesh|AddInstance _grassism InstanceTransform false)
      (Utilities|Array|Add (Variables|/Script/Engine.ActorComponent|GetComponentTags _grassism) "Grass"))
    (:NewEnumerator1
      (Components|InstancedStaticMesh|AddInstance _sandism InstanceTransform false)
      (Utilities|Array|Add (Variables|/Script/Engine.ActorComponent|GetComponentTags _sandism) "Sand"))
    (:NewEnumerator2
      (Components|InstancedStaticMesh|AddInstance _mountainism InstanceTransform false)
      (Utilities|Array|Add (Variables|/Script/Engine.ActorComponent|GetComponentTags _mountainism) "Mountain"))))