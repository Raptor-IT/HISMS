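; BP_ColourActor is a workshop premade actor that places coloured cubes as instances of a single instanced static mesh.
; Its construction script clears CubeISM and adds a local-space instance for each transform in the Instances array.
; Per-instance custom data carries each cube's RGB, either random per channel when RandomColour is set or taken from the SetColour vector.
; The event graph is empty, so all work happens at construction.
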(event EventBeginPlay)

(event Collision|EventActorBeginOverlap
  (params (OtherActor :type Actor%20Object%20Reference)))

(event EventTick
  (params (DeltaSeconds :type Float%20%28single-precision%29)))

(fn ConstructionScript
  (bind _returnvalue (Math|Random|RandomFloat))
  (bind _cubeism (Variables|Default|GetCubeISM))
  (bind _set_colour (Variables|Default|GetSet%20Colour))
  (bind (_x _y _z) (Math|Vector|BreakVector _set_colour))
  (Components|InstancedStaticMesh|ClearInstances _cubeism)
  (for _array_element (Variables|Default|GetInstances)
    (bind _returnvalue_2 (Components|InstancedStaticMesh|AddInstance _cubeism _array_element false))
    (if (Variables|Default|GetRandom%20Colour%20?%20)
      (Components|InstancedStaticMesh|SetCustomDataValue _cubeism _returnvalue_2 0 _returnvalue true) ; Red (R)
      (Components|InstancedStaticMesh|SetCustomDataValue _cubeism _returnvalue_2 1 _returnvalue true) ; Green (G)
      (Components|InstancedStaticMesh|SetCustomDataValue _cubeism _returnvalue_2 2 _returnvalue true) ; Blue (B)
      (else
        (Components|InstancedStaticMesh|SetCustomDataValue _cubeism _returnvalue_2 0 _x true) ; Red (R)
        (Components|InstancedStaticMesh|SetCustomDataValue _cubeism _returnvalue_2 1 _y true) ; Green (G)
        (Components|InstancedStaticMesh|SetCustomDataValue _cubeism _returnvalue_2 2 _z true) ; Blue (B)
      ))))